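; BP_MainCharacter2 is a player character that moves in steps on a small bounded grid and can toggle an inventory.
; Directional grid inputs check the actor's X or Y location against fixed limits, then offset the capsule one cell in world space.
; The OpenInventory input calls ToggleInventory on BPInventory.
; Free axis movement and an older HUD animation toggle remain as disconnected, unused nodes.
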(event EventBeginPlay)

(event Collision|EventActorBeginOverlap
  (params (OtherActor :type Actor%20Object%20Reference)))

(event EventTick
  (params (DeltaSeconds :type Float%20%28single-precision%29)))

(event Input|ActionEvents|InputActionOpenInventory
  (params (Key :type Key%20Structure :default "None"))
  (:Pressed
    (Default|ToggleInventory (Variables|Default|GetBP_Inventory))))

(event Input|ActionEvents|InputActionMoveRight_Grid
  (params (Key :type Key%20Structure :default "None"))
  ;[1 1 1] Movement Inputs
  (:Pressed
    (if (< (.x (.location (Transformation|GetActorTransform))) 2e+02)
      (Transformation|AddWorldOffset (Variables|Collision|GetCapsuleComponent) (Math|Vector|MakeVector 1e+02 0.0 0.0) false false))))

(event Input|ActionEvents|InputActionMoveLeft_Grid
  (params (Key :type Key%20Structure :default "None"))
  ;[1 1 1] Movement Inputs
  (:Pressed
    (if (> (.x (.location (Transformation|GetActorTransform))) 0.0)
      (Transformation|AddWorldOffset (Variables|Collision|GetCapsuleComponent) (Math|Vector|MakeVector -1e+02 0.0 0.0) false false))))

(event Input|ActionEvents|InputActionMoveUp_Grid
  (params (Key :type Key%20Structure :default "None"))
  ;[1 1 1] Movement Inputs
  (:Pressed
    (if (> (.y (.location (Transformation|GetActorTransform))) 0.0)
      (Transformation|AddWorldOffset (Variables|Collision|GetCapsuleComponent) (Math|Vector|MakeVector 0.0 -1e+02 0.0) false false))))

(event Input|ActionEvents|InputActionMoveDown_Grid
  (params (Key :type Key%20Structure :default "None"))
  ;[1 1 1] Movement Inputs
  (:Pressed
    (if (< (.y (.location (Transformation|GetActorTransform))) 2e+02)
      (Transformation|AddWorldOffset (Variables|Collision|GetCapsuleComponent) (Math|Vector|MakeVector 0.0 1e+02 0.0) false false))))

(event Input|AxisEvents|InputAxisMoveForward
  (params (AxisValue :type Float%20%28single-precision%29))
  ;[1 1 1] Movement Inputs
)

(event Input|AxisEvents|InputAxisMoveRight
  (params (AxisValue :type Float%20%28single-precision%29))
  ;[1 1 1] Movement Inputs
)

(fn ConstructionScript)