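; Inventory actor component whose only implemented logic toggles the inventory window open and closed.
; Opening creates a BP_InventoryWindow bound to the component, adds it auto-sized to the HUD's InventoryCanvas via BP_PlayerController, plays the open animation and switches to UI-only input with a cursor.
; Closing removes the window, restores game-only input, hides the cursor and prints a debug message.
; Centering and positioning nodes are present but disconnected.
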(event EventBeginPlay)

(event EventTick
  (params (DeltaSeconds :type Float%20%28single-precision%29)))

(fn ToggleInventory
  (bind _returnvalue (Game|GetPlayerController 0))
  (bind _returnvalue_2 (Game|GetPlayerController 0))
  (bind _returnvalue_3 (Game|GetPlayerController 0))
  (bind _asbp_player_controller (Utilities|Casting|CastToBP_PlayerController _returnvalue_2))
  (bind _hudwidget (Variables|/Game/Blueprints/BP_PlayerController.BP_PlayerController_C|GetHudWidget _asbp_player_controller))
  (Variables|Default|GetInventoryWindow
    (:then
      (Widget|RemovefromParent (Variables|Default|GetInventoryWindow))
      (Variables|Default|SetInventoryWindow 0)
      (Input|SetInputModeGameOnly _returnvalue)
      (Variables|/Script/Engine.PlayerController|SetbShowMouseCursor _returnvalue false)
      (Development|PrintString "Toggled To Close!" true true "(R=0.000000,G=0.660000,B=1.000000,A=1.000000)" 1e+01))
    (:else
      (bind _returnvalue_4 (UserInterface|CreateWidget "/Game/Widgets/InventoryUI/BP_InventoryWindow.BP_InventoryWindow_C" 0 self))
      (Variables|Default|SetInventoryWindow _returnvalue_4)
      (bind _asbp_player_controller_2 (Utilities|Casting|CastToBP_PlayerController (Game|GetPlayerController 0)))
      (bind _returnvalue_5 (Class|CanvasPanel|AddChildtoCanvas (Variables|/Game/Widgets/BP_HUD.BP_HUD_C|GetInventoryCanvas (Variables|/Game/Blueprints/BP_PlayerController.BP_PlayerController_C|GetHudWidget _asbp_player_controller_2)) (Variables|Default|GetInventoryWindow)))
      (Class|CanvasPanelSlot|SetAutoSize _returnvalue_5 true)
      (UserInterface|Animation|PlayAnimation _hudwidget (Variables|/Game/Widgets/BP_HUD.BP_HUD_C|GetOpenInventoryAnimation _hudwidget) 0.0 1 "Forward" 1.0 false)
      (Input|SetInputModeUIOnly _returnvalue_3 (Variables|Default|GetInventoryWindow) "LockAlways")
      (Variables|/Script/Engine.PlayerController|SetbShowMouseCursor _returnvalue_3 true))))